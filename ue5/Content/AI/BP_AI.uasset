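; BP_AI is the pet AI character, which registers itself and its AI controller with tangoGameInstance on BeginPlay.
; When PawnSensing sees an ALS_MainCharacter, it sets the hasSeenPlayer? Blackboard key to true; nothing here clears it.
; Leftover nodes that print and increment the tamedScale key are disconnected and never run.
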(event OnSeePawn(PawnSensing)
  (params (Pawn :type Pawn%20Object%20Reference))
  (Utilities|Casting|CastToALS_MainCharacter Pawn)
  (AI|Components|Blackboard|SetValueasBool (AI|GetBlackboard (AI|GetAIController self)) (Utilities|Name|MakeLiteralName "hasSeenPlayer?") true))

(event Custom|SpawnText)

(event EventTick
  (params (DeltaSeconds :type Float%20%28single-precision%29)))

(event EventBeginPlay
  (bind _astango_game_instance (Utilities|Casting|CastTotangoGameInstance (Game|GetGameInstance)))
  (Variables|/Game/ApeCoin/tangoGameInstance.tangoGameInstance_C|SetpetAIBP _astango_game_instance self)
  (bind _output_get (Variables|Default|SetgameInst _astango_game_instance))
  (Variables|/Game/ApeCoin/tangoGameInstance.tangoGameInstance_C|SetpetAIController _output_get (AI|GetAIController 0)))

(fn ConstructionScript)